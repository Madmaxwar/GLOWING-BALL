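; BP_cannon is a cannon that fires BP_Projectile automatically and repeatedly from the start of play.
; After a fire-rate delay, it spawns a scaled projectile at the SpwanPoint component's world transform and plays the CannonFire timeline.
; The timeline's Fire track drives the Cannon component's relative location, and its Cannon Fired event track loops back to the delay for the next shot.
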(event `self.ReceiveBeginPlay`
  (`KismetSystemLibrary.Delay` (`self.cannonfirerate`) :!label _label)
  (`self.Spawn projectile`)
  (bind (_direction _fire) (`Timeline|Cannon Fire` :!via `PlayFromStart`)
    (:`Update`
      (`self.Move cannon ` _fire))
    (:`cannon fired`
      (goto _label))))

(fn `Move cannon `
  (params (NewLocation_Y :type "Float (double-precision)"))
  (`SceneComponent.K2_SetRelativeLocation` (`self.cannon`) (`KismetMathLibrary.MakeVector` 0.0 NewLocation_Y) false false))

(fn `Spawn projectile`
  (bind _spwanpoint (`self.SpwanPoint`))
  (`|SpawnActorFromClass` "/Game/BP/BP_Projectile.BP_Projectile_C" (`KismetMathLibrary.MakeTransform` (`SceneComponent.K2_GetComponentLocation` _spwanpoint) (`SceneComponent.K2_GetComponentRotation` _spwanpoint) (`KismetMathLibrary.Conv_DoubleToVector` (`self.Projectile Scale`))) "Undefined" "OverrideRootScale" null null))

(fn `UserConstructionScript`)