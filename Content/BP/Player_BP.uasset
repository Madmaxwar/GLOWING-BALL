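; Player Blueprint for a rolling-sphere character that restarts the current level when it takes any damage.
; W/S and A/D axis inputs apply torque to the Sphere around Y and X to roll it.
; The camera fades in on BeginPlay; damage starts a one-time fade-out with audio, then reopens the level immediately, without waiting for the fade.
; The PlayerSpringARM function sets the camera boom's length and world pitch, zeroing yaw and roll.
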(event `self.ReceiveAnyDamage`
  (params (Damage :type "Float (single-precision)") (DamageType :type "DamageType Object Reference") (InstigatedBy :type "Controller Object Reference") (DamageCauser :type "Actor Object Reference"))
  (`/Engine/EditorBlueprintResources/StandardMacros.DoOnce` false
    (:`Completed`
      (`PlayerCameraManager.StartCameraFade` :`self` (`GameplayStatics.GetPlayerCameraManager` 0) :`ToAlpha` 1.0 :`Duration` 2.0 :`bShouldFadeAudio` true)
      (bind _returnvalue (`GameplayStatics.GetCurrentLevelName` true))
      (`GameplayStatics.OpenLevel` (`KismetStringLibrary.Conv_StringToName` _returnvalue)))))

(event `self.ReceiveBeginPlay`
  (`PlayerCameraManager.StartCameraFade` :`self` (`GameplayStatics.GetPlayerCameraManager` 0) :`FromAlpha` 1.0 :`Duration` 3.0))

(event `InputAxis|W/S`
  (params (AxisValue :type "Float (single-precision)"))
  (`PrimitiveComponent.AddTorqueInRadians` (`self.Sphere`) (`KismetMathLibrary.MakeVector` 0.0 (* AxisValue 20000.0)) "None" false))

(event `InputAxis|A/D`
  (params (AxisValue :type "Float (single-precision)"))
  (`PrimitiveComponent.AddTorqueInRadians` (`self.Sphere`) (`KismetMathLibrary.MakeVector` (* AxisValue 20000.0)) "None" false))

(fn `player Spring ARM`
  (params (distance :type "Float (double-precision)") (pitch :type "Float (double-precision)"))
  (bind _springarm (`self.SpringArm`))
  (set `SpringArmComponent.TargetArmLength` distance _springarm)
  (`SceneComponent.K2_SetWorldRotation` _springarm (`KismetMathLibrary.MakeRotator` 0.0 pitch) false false))

(fn `UserConstructionScript`)