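; Crystal pickup actor that flies to the player and disappears when the player pawn overlaps it.
; The overlap stores the crystal's location as a start point, then plays a timeline that lerps it toward the pawn's current location each update, so it tracks a moving player.
; The actor destroys itself when the timeline finishes; no score or inventory change happens here.
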(event `self.ReceiveActorBeginOverlap`
  (params (OtherActor :type "Actor Object Reference"))
  (if (== OtherActor (`GameplayStatics.GetPlayerPawn` 0))
    (set `self.LerpStartlocation` (`self.K2_GetActorLocation`))
    (bind (_direction _newtrack_0) (`Timeline|Alpha Blend Timeline`)
      (:`Update`
        (`self.K2_SetActorLocation` (`KismetMathLibrary.VLerp` (`self.LerpStartlocation`) (`self.K2_GetActorLocation` (`GameplayStatics.GetPlayerPawn` 0)) _newtrack_0)))
      (:`Finished`
        (`self.K2_DestroyActor`)))))

(fn `UserConstructionScript`)